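; Race manager that runs a timed run through ordered checkpoints and keeps the best run's split times.
; On BeginPlay it orders all BP_Checkpoint actors by Index, creates the WB_Game HUD and starts a looping timer.
; Each checkpoint event records a split, shows it against the saved best and activates the next checkpoint.
; The last checkpoint stops the timer and saves splits to SG_PlayerData if none exist or the total is faster.
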(event `self.ReceiveBeginPlay`
  (`|ExecutionSequence`
    (:`then_0`
      (`self.GetAllCheckpointActor`)
      (bind _returnvalue (`|CreateWidget` "/Game/01-Blueprints/Widget/WB_Game.WB_Game_C" (`GameplayStatics.GetPlayerController` 0)))
      (bind _output_get (set `self.GameWidget` _returnvalue))
      (`UserWidget.AddToViewport` _output_get 0))
    (:`then_1`
      (bind _returnvalue_2 (`KismetSystemLibrary.K2_SetTimerDelegate` (delegate `GameTimer Event`) 0.01 true))
      (set `self.TimerHandle` _returnvalue_2))))

(event `GameTimer Event`
  (bind _output_get (set `self.Timer` (+ (`self.Timer`) 0.01)))
  (`/Game/01-Blueprints/Widget/WB_Game.SetTimerText` (`self.GameWidget`) _output_get))

(event `OnCheckpointReceived`
  (`KismetArrayLibrary.Array_Add` (`self.CheckpointTime`) (`self.Timer`))
  (`|ExecutionSequence`
    (:`then_0`
      (bind _returnvalue (`GameplayStatics.DoesSaveGameExist` "PlayerData"))
      (if _returnvalue
        (bind _returnvalue_2 (`GameplayStatics.LoadGameFromSlot` "PlayerData"))
        (bind _assg_player_data (cast `/Game/01-Blueprints/SG_PlayerData` _returnvalue_2))
        (`/Game/01-Blueprints/Widget/WB_Game.SetIntervalleText` (`self.GameWidget`) (`self.Timer`) (`|GetArrayItem` (`/Game/01-Blueprints/SG_PlayerData.CheckpointTime` _assg_player_data) (`self.ActualCheckpointIndex`)))))
    (:`then_1`
      (if (< (+ (`self.ActualCheckpointIndex`) 1) (`KismetArrayLibrary.Array_Length` (`self.CheckpointList`)))
        (bind _output_get (set `self.ActualCheckpointIndex` (+ (`self.ActualCheckpointIndex`) 1)))
        (bind _output (`|GetArrayItem` (`self.CheckpointList`) _output_get))
        (set `PrimitiveComponent.bGenerateOverlapEvents` true (`/Game/01-Blueprints/Actor/BP_Checkpoint.Box` _output))
        (`SceneComponent.SetVisibility` (`/Game/01-Blueprints/Actor/BP_Checkpoint.Disc_CD15932C` _output) true false)
        (else
          (`KismetSystemLibrary.K2_ClearAndInvalidateTimerHandle` (`self.TimerHandle`))
          (`self.Save Checkpoint`))))))

(fn `GetAllCheckpointActor`
  (bind _output (`|GetArrayItem` (`self.CheckpointList`)))
  (bind _outactors (`GameplayStatics.GetAllActorsOfClass` "/Game/01-Blueprints/Actor/BP_Checkpoint.BP_Checkpoint_C"))
  (for _array_element _outactors
    (`KismetArrayLibrary.Array_Set` (`self.CheckpointList`) (`/Game/01-Blueprints/Actor/BP_Checkpoint.Index` _array_element) _array_element true)
    (add `/Game/01-Blueprints/Actor/BP_Checkpoint.OnCheckpointReached` _array_element (`|CreateDelegate` :!event `OnCheckpointReceived`)))
  (set `PrimitiveComponent.bGenerateOverlapEvents` true (`/Game/01-Blueprints/Actor/BP_Checkpoint.Box` _output))
  (`SceneComponent.SetVisibility` (`/Game/01-Blueprints/Actor/BP_Checkpoint.Disc_CD15932C` _output) true false))

(fn `Lose`)

(fn `Save Checkpoint`
  (bind _checkpointtime (`self.CheckpointTime`))
  (bind _returnvalue (`GameplayStatics.DoesSaveGameExist` "PlayerData"))
  (if _returnvalue
    (bind _returnvalue_2 (`GameplayStatics.LoadGameFromSlot` "PlayerData"))
    (bind _assg_player_data (cast `/Game/01-Blueprints/SG_PlayerData` _returnvalue_2))
    (bind _checkpointtime_2 (`/Game/01-Blueprints/SG_PlayerData.CheckpointTime` _assg_player_data))
    (if (< (`|GetArrayItem` _checkpointtime (`KismetArrayLibrary.Array_LastIndex` _checkpointtime)) (`|GetArrayItem` _checkpointtime_2 (`KismetArrayLibrary.Array_LastIndex` _checkpointtime_2)))
      (set `/Game/01-Blueprints/SG_PlayerData.CheckpointTime` (`self.CheckpointTime`) _assg_player_data)
      (`GameplayStatics.SaveGameToSlot` _assg_player_data "PlayerData"))
    (else
      (bind _returnvalue_3 (`GameplayStatics.CreateSaveGameObject` "/Game/01-Blueprints/SG_PlayerData.SG_PlayerData_C"))
      (set `/Game/01-Blueprints/SG_PlayerData.CheckpointTime` (`self.CheckpointTime`) _returnvalue_3)
      (`GameplayStatics.SaveGameToSlot` _returnvalue_3 "PlayerData"))))

(fn `UserConstructionScript`)