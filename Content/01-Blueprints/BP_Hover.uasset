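; Player hover vehicle pawn with thrust, steering, limited boost and mouse- or gamepad-aimed shooting.
; Enhanced Input feeds target speeds to BPMovementComponent; boost multiplies thrust, drains a HUD meter by timer and drives jet effects and FOV.
; Shots trace through the cursor to aim physics-impulse bullets, while velocity scales speed lines, camera shake and engine pitch.
; Functions handle boost pads, refills, input toggling and switching gravity with camera inheritance.
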(event `self.ReceiveBeginPlay`
  (bind _returnvalue (`GameplayStatics.GetPlayerController` 0))
  (bind _vehicle (`self.Vehicle`))
  (bind _returnvalue_2 (pcsubsystem `EnhancedInputLocalPlayerSubsystem` (`GameplayStatics.GetPlayerController` 0)))
  (`/Engine/EditorBlueprintResources/StandardMacros.IsValid` _returnvalue_2
    (:`Is Valid`
      (`EnhancedInputSubsystemInterface.AddMappingContext` _returnvalue_2 "/Game/03-Inputs/IMC_Hover.IMC_Hover" 0 (struct))
      (`EnhancedInputSubsystemInterface.AddMappingContext` _returnvalue_2 "/Game/03-Inputs/IMC_Pause.IMC_Pause" 0 (struct))
      (set `PlayerController.CurrentMouseCursor` "Crosshairs" _returnvalue)
      (set `PlayerController.bShowMouseCursor` true _returnvalue)
      (bind _returnvalue_3 (`|CreateWidget` "/Game/01-Blueprints/Widget/WB_Player.WB_Player_C" (`GameplayStatics.GetPlayerController` 0)))
      (bind _output_get (set `self.PlayerWidget` _returnvalue_3))
      (`UserWidget.AddToViewport` _output_get 0)
      (`/Game/01-Blueprints/Widget/WB_Player.SetBoost` _output_get (`self.BoostUnit`))
      (bind _returnvalue_4 (`LegacyCameraShake.StartLegacyCameraShake` (`GameplayStatics.GetPlayerCameraManager` 0) "/Game/07-FX/VFX/LCS_CameraShakeRoad.LCS_CameraShakeRoad_C"))
      (set `self.RoadCameraShake` _returnvalue_4)
      (`self.Gravity`)
      (bind _returnvalue_5 (`|CreateWidget` "/Game/01-Blueprints/Widget/WB_PauseMenu.WB_PauseMenu_C"))
      (set `self.PauseMenu` _returnvalue_5)
      (`AudioComponent.Stop` (`self.Jet`))
      (bind _returnvalue_6 (`PrimitiveComponent.CreateDynamicMaterialInstance` _vehicle 0 (`PrimitiveComponent.GetMaterial` _vehicle 0) "None"))
      (set `self.DynMaterial` _returnvalue_6))))

(event `EnhancedInput|/Game/03-Inputs/Actions/IA_Thurst`
  (params (ActionValue :type "Float (double-precision)") (ElapsedSeconds :type "Float (double-precision)") (TriggeredSeconds :type "Float (double-precision)") (InputAction :type "InputAction Object Reference" :default "/Game/03-Inputs/Actions/IA_Thurst.IA_Thurst"))
  (bind _bp_movementcomponent (`self.BP_MovementComponent`))
  (:`Triggered`
    (set `/Game/01-Blueprints/Components/BP_MovementComponent.TargetSpeed` (* ActionValue (`self.MaxSpeed`) (`self.BoostMultiplier`)) _bp_movementcomponent))
  (:`Started`
    (set `self.engineStarted` true))
  (:`Completed`
    (set `/Game/01-Blueprints/Components/BP_MovementComponent.TargetSpeed` 0.0 _bp_movementcomponent)))

(event `EnhancedInput|/Game/03-Inputs/Actions/IA_Steer`
  (params (ActionValue :type "Float (double-precision)") (ElapsedSeconds :type "Float (double-precision)") (TriggeredSeconds :type "Float (double-precision)") (InputAction :type "InputAction Object Reference" :default "/Game/03-Inputs/Actions/IA_Steer.IA_Steer"))
  (bind _bp_movementcomponent (`self.BP_MovementComponent`))
  (:`Triggered`
    (set `/Game/01-Blueprints/Components/BP_MovementComponent.TargetAngularSpeed` (* ActionValue (`self.MaxAngularSpeed`)) _bp_movementcomponent))
  (:`Completed`
    (set `/Game/01-Blueprints/Components/BP_MovementComponent.TargetAngularSpeed` 0.0 _bp_movementcomponent)))

(event `CustomEvent`
  (bind _output_get (set `self.BoostUnit` (- (`self.BoostUnit`) 0.4)))
  (`/Game/01-Blueprints/Widget/WB_Player.SetBoost` (`self.PlayerWidget`) _output_get))

(event `EnhancedInput|/Game/03-Inputs/Actions/IA_Boost`
  (params (ActionValue :type Boolean) (ElapsedSeconds :type "Float (double-precision)") (TriggeredSeconds :type "Float (double-precision)") (InputAction :type "InputAction Object Reference" :default "/Game/03-Inputs/Actions/IA_Boost.IA_Boost"))
  (bind _jet (`self.Jet`))
  (bind _jet_2 (`self.Jet`))
  (:`Started`
    (if (> (`self.BoostUnit`) 0.0)
      (if (not (`AudioComponent.IsPlaying` _jet_2))
        (`FXSystemComponent.SetFloatParameter` (`self.NiagaraHoverBR`) "Red" 1.0)
        (`FXSystemComponent.SetFloatParameter` (`self.NiagaraHoverBL`) "Red" 1.0)
        (`FXSystemComponent.SetFloatParameter` (`self.NiagaraHoverBL`) "Other" 0.0)
        (`FXSystemComponent.SetFloatParameter` (`self.NiagaraHoverBR`) "Other" 0.0)
        (`AudioComponent.Play` _jet_2 0.0))
      (set `self.BoostMultiplier` 3.0)
      (bind _returnvalue (`KismetSystemLibrary.K2_SetTimerDelegate` (delegate `CustomEvent`) 0.01 true))
      (set `self.BoostTimerHandle` _returnvalue)
      (else
        (set `self.BoostUnit` 0.0 :!label _label)
        (set `self.BoostMultiplier` 1.0 :!label _label_2)
        (if (`AudioComponent.IsPlaying` _jet)
          (`AudioComponent.Stop` _jet)
          (`FXSystemComponent.SetFloatParameter` (`self.NiagaraHoverBR`) "Red" 0.0)
          (`FXSystemComponent.SetFloatParameter` (`self.NiagaraHoverBL`) "Red" 0.0)
          (`FXSystemComponent.SetFloatParameter` (`self.NiagaraHoverBL`) "Other" 1.0)
          (`FXSystemComponent.SetFloatParameter` (`self.NiagaraHoverBR`) "Other" 1.0))
        (`KismetSystemLibrary.K2_ClearAndInvalidateTimerHandle` (`self.BoostTimerHandle`))
        (if (!= (`CameraComponent.FieldOfView` (`self.Camera`)) (`self.FOVnormal`))
          (bind (_direction _newtrack_1) (`Timeline|Timeline` :!via `Reverse` :!label _label_3)
            (:`Update`
              (`CameraComponent.SetFieldOfView` (`self.Camera`) (`KismetMathLibrary.Lerp` (`self.FOVnormal`) (`self.FOVBoost`) _newtrack_1))))
          (else
            (set `self.SpeedLinePower` 1.0)
            (goto _label_3 :!via `Stop`))))))
  (:`Ongoing`
    (if (> (`self.BoostUnit`) 0.0)
      (if (!= (`CameraComponent.FieldOfView` (`self.Camera`)) (`self.FOVBoost`))
        (set `self.SpeedLinePower` 2.0)
        (goto _label_3)
        (else
          (goto _label_3 :!via `Stop`)))
      (else
        (goto _label))))
  (:`Completed`
    (goto _label_2)))

(event `ResetBoost`
  (goto _label_2))

(event `EnhancedInput|/Game/03-Inputs/Actions/IA_Shoot`
  (params (ActionValue :type "Vector2D Structure") (ElapsedSeconds :type "Float (double-precision)") (TriggeredSeconds :type "Float (double-precision)") (InputAction :type "InputAction Object Reference" :default "/Game/03-Inputs/Actions/IA_Shoot.IA_Shoot"))
  (bind _returnvalue (`SceneComponent.K2_GetComponentLocation` (`self.Camera`)))
  (bind _returnvalue_2 (`SceneComponent.K2_GetComponentLocation` (`self.BulletSpawn`)))
  (bind _returnvalue_3 (`SceneComponent.K2_GetComponentLocation` (`self.BulletSpawn`)))
  (:`Started`
    (if (`self.CanShoot`)
      (`GameplayStatics.PlaySoundAtLocation` "/Game/07-FX/SFX/laser-104024.laser-104024" (`SceneComponent.K2_GetComponentLocation` (`self.BulletSpawn`)) (struct) 1.0 1.0 0.0 null null null null)
      (bind (_outhit _returnvalue_4) (`KismetSystemLibrary.LineTraceSingle` :`Start` _returnvalue :`End` (+ _returnvalue (* (`.WorldDirection` (`PlayerController.DeprojectMousePositionToWorld` (`GameplayStatics.GetPlayerController` 0))) 25000.0)) :`TraceChannel` "TraceTypeQuery1" :`DrawDebugType` (select `bool` false :`true` "Persistent" :!type "EDrawDebugTrace Enum")))
      (if _returnvalue_4
        (bind _returnvalue_5 (`|SpawnActorFromClass` "/Game/01-Blueprints/Actor/BP_Bullet.BP_Bullet_C" (`KismetMathLibrary.MakeTransform` _returnvalue_2 (`KismetMathLibrary.FindLookAtRotation` _returnvalue_2 (`.Location` (`GameplayStatics.BreakHitResult` _outhit)))) "Undefined" "MultiplyWithRoot" null null))
        (`PrimitiveComponent.AddImpulse` (`/Game/01-Blueprints/Actor/BP_Bullet.Sphere` _returnvalue_5) (* (`KismetMathLibrary.GetDirectionUnitVector` _returnvalue_2 (`.Location` (`GameplayStatics.BreakHitResult` _outhit))) (`self.BulletSpeed`)) "None" false)
        (`self.SetLifeSpan` _returnvalue_5 5.0)
        (else
          (bind _returnvalue_6 (`|SpawnActorFromClass` "/Game/01-Blueprints/Actor/BP_Bullet.BP_Bullet_C" (`KismetMathLibrary.MakeTransform` _returnvalue_3 (`KismetMathLibrary.FindLookAtRotation` _returnvalue_3 (`.TraceEnd` (`GameplayStatics.BreakHitResult` _outhit)))) "Undefined" "MultiplyWithRoot" null null))
          (`PrimitiveComponent.AddImpulse` (`/Game/01-Blueprints/Actor/BP_Bullet.Sphere` _returnvalue_6) (* (`KismetMathLibrary.GetDirectionUnitVector` _returnvalue_3 (`.TraceEnd` (`GameplayStatics.BreakHitResult` _outhit))) (`self.BulletSpeed`)) "None" false)
          (`self.SetLifeSpan` _returnvalue_6 5.0))))))

(event `self.ReceiveTick`
  (params (DeltaSeconds :type "Float (single-precision)"))
  (bind _motor (`self.Motor`))
  (bind _motor_2 (`self.Motor`))
  (bind _returnvalue (`|EnumEquality` (`AudioComponent.GetPlayState` _motor) "Playing"))
  (bind _returnvalue_2 (/ (`KismetMathLibrary.VSize` (`SceneComponent.GetComponentVelocity` (`self.Vehicle`))) 500.0))
  (bind _returnvalue_3 (* _returnvalue_2 (`self.SpeedLinePower`)))
  (`FXSystemComponent.SetFloatParameter` (`self.Niagara`) "SpawnRateUser" _returnvalue_3)
  (set `CameraShakeBase.ShakeScale` _returnvalue_3 (`self.RoadCameraShake`))
  (if (`self.engineStarted`)
    (`AudioComponent.SetPitchMultiplier` _motor (+ (/ _returnvalue_2 50.0) 1.0))
    (if (not _returnvalue)
      (`AudioComponent.Play` _motor_2 0.0))
    (elif _returnvalue
      (`AudioComponent.Stop` _motor_2))))

(event `EnhancedInput|/Game/03-Inputs/Actions/IA_MoveCursorGamePad`
  (params (ActionValue :type "Vector2D Structure") (ElapsedSeconds :type "Float (double-precision)") (TriggeredSeconds :type "Float (double-precision)") (InputAction :type "InputAction Object Reference" :default "/Game/03-Inputs/Actions/IA_MoveCursorGamePad.IA_MoveCursorGamePad"))
  (bind (_x _y) (`KismetMathLibrary.BreakVector2D` ActionValue))
  (bind (_locationx _locationy) (`PlayerController.GetMousePosition` (`GameplayStatics.GetPlayerController` 0)))
  (:`Triggered`
    (`PlayerController.SetMouseLocation` (`GameplayStatics.GetPlayerController` 0) (`KismetMathLibrary.Round` (+ (* _x 10.0) _locationx)) (`KismetMathLibrary.Round` (+ (* _y 10.0) _locationy)))))

(event `EnhancedInput|/Game/03-Inputs/Actions/IA_Pause`
  (params (ActionValue :type Boolean) (ElapsedSeconds :type "Float (double-precision)") (TriggeredSeconds :type "Float (double-precision)") (InputAction :type "InputAction Object Reference" :default "/Game/03-Inputs/Actions/IA_Pause.IA_Pause"))
  (:`Triggered`
    (`GameplayStatics.SetGamePaused` true)
    (`UserWidget.AddToViewport` (`self.PauseMenu`) 0)))

(fn `AddBoost`
  (params (Value :type "Float (double-precision)"))
  (bind _returnvalue (+ Value (`self.BoostUnit`)))
  (if (<= _returnvalue 100.0)
    (set `self.BoostUnit` _returnvalue)
    (else
      (set `self.BoostUnit` 100.0)))
  (`/Game/01-Blueprints/Widget/WB_Player.SetBoost` (`self.PlayerWidget`) (`self.BoostUnit`)))

(fn `BoostPads`
  (bind _vehicle (`self.Vehicle`))
  (`PrimitiveComponent.AddImpulse` _vehicle (* (`SceneComponent.GetForwardVector` _vehicle) (`self.BoostPadForce`)) "None" true))

(fn `DisableMapping`
  (bind _bp_movementcomponent (`self.BP_MovementComponent`))
  (bind _returnvalue (pcsubsystem `EnhancedInputLocalPlayerSubsystem` (`GameplayStatics.GetPlayerController` 0)))
  (`/Engine/EditorBlueprintResources/StandardMacros.IsValid` _returnvalue
    (:`Is Valid`
      (`EnhancedInputSubsystemInterface.RemoveMappingContext` _returnvalue "/Game/03-Inputs/IMC_Hover.IMC_Hover" (struct))
      (`self.ResetBoost`)
      (set `/Game/01-Blueprints/Components/BP_MovementComponent.TargetSpeed` 0.0 _bp_movementcomponent)
      (set `/Game/01-Blueprints/Components/BP_MovementComponent.TargetAngularSpeed` 0.0 _bp_movementcomponent))))

(fn `EnableMapping`
  (bind _returnvalue (pcsubsystem `EnhancedInputLocalPlayerSubsystem` (`GameplayStatics.GetPlayerController` 0)))
  (`/Engine/EditorBlueprintResources/StandardMacros.IsValid` _returnvalue
    (:`Is Valid`
      (`EnhancedInputSubsystemInterface.AddMappingContext` _returnvalue "/Game/03-Inputs/IMC_Hover.IMC_Hover" 0 (struct)))))

(fn `Gravity`
  (bind _bp_gravitycomponent (`self.BP_GravityComponent`))
  (bind _springarm (`self.SpringArm`))
  (bind _isenabled (`/Game/01-Blueprints/Components/BP_GravityComponent.IsEnabled` _bp_gravitycomponent))
  (bind _returnvalue (not _isenabled))
  (`PrimitiveComponent.SetEnableGravity` (`self.Vehicle`) _isenabled)
  (bind _output_get (set `SpringArmComponent.bInheritPitch` _returnvalue _springarm))
  (set `SpringArmComponent.bInheritRoll` _output_get _springarm)
  (set `/Game/01-Blueprints/Components/BP_GravityComponent.IsEnabled` _returnvalue _bp_gravitycomponent))

(fn `UserConstructionScript`)